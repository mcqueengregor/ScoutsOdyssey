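; BP_Philbert is an actor, apparently a character prefab, with a dialogue component, a speech bubble and an overlap collider.
; Overlapping the collider starts its ActorSequence looping, and ending the overlap stops it.
; Tick polls the dialogue component's HasTriggered flag and hides the speech bubble once it is set, with no logic to show it again.
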(event OnComponentBeginOverlap(OverlapCollider)
  (params (OverlappedComponent :type Primitive%20Component%20Object%20Reference) (OtherActor :type Actor%20Object%20Reference) (OtherComp :type Primitive%20Component%20Object%20Reference) (OtherBodyIndex :type Integer) (bFromSweep :type Boolean) (SweepResult :type Hit%20Result%20Structure%20%28by%20ref%29))
  (bind _actorsequence (Variables|Default|GetActorSequence))
  (bind _sequenceplayer (Variables|/Script/ActorSequence.ActorSequenceComponent|GetSequencePlayer _actorsequence))
  (Utilities|IsValid _sequenceplayer
    (:Is%20Valid
      (Class|MovieSceneSequencePlayer|PlayLooping _sequenceplayer -1))))

(event OnComponentEndOverlap(OverlapCollider)
  (params (OverlappedComponent :type Primitive%20Component%20Object%20Reference) (OtherActor :type Actor%20Object%20Reference) (OtherComp :type Primitive%20Component%20Object%20Reference) (OtherBodyIndex :type Integer))
  (bind _actorsequence (Variables|Default|GetActorSequence))
  (bind _sequenceplayer (Variables|/Script/ActorSequence.ActorSequenceComponent|GetSequencePlayer _actorsequence))
  (Utilities|IsValid _sequenceplayer
    (:Is%20Valid
      (Sequencer|Player|Stop _sequenceplayer :!class /Script/MovieScene.MovieSceneSequencePlayer))))

(event EventBeginPlay)

(event Collision|EventActorBeginOverlap
  (params (OtherActor :type Actor%20Object%20Reference)))

(event EventTick
  (params (DeltaSeconds :type Float%20%28single-precision%29))
  (bind _speechbubble (Variables|Default|GetSpeechBubble))
  (if (Variables|/Script/ScoutsOdyssey.DialogueComponent|GetHasTriggered (Variables|Default|GetBP_DialogueComponent))
    (if (not (Variables|/Script/Engine.SceneComponent|GetbHiddenInGame _speechbubble))
      (Development|SetHiddeninGame _speechbubble true false))))

(fn ConstructionScript)