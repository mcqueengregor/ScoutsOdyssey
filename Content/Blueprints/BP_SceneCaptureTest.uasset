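; BP_SceneCaptureTest is a test actor that captures only the player pawn's mesh through a SceneCaptureComponent2D.
; On BeginPlay it caches BP_PlayerPawn and adds its MeshComponent as a show-only component.
; Each tick it snaps the capture to the camera of the pawn's LastEnteredSection, copying transform and FOV so the render matches that stage camera angle.
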(event EventBeginPlay
  ;[1 1 1] Store reference to player pawn in the world:
  (bind _asbp_player_pawn (Utilities|Casting|CastToBP_PlayerPawn (Game|Player|GetPlayerPawn 0))
    (:then
      (bind _output_get (Variables|Default|SetPawnRef _asbp_player_pawn))
      ;[1 1 1] Mark player's sprite as the only thing being rendered by the SceneCaptureComponent:
      (Rendering|SceneCapture|ShowOnlyComponent (Variables|Default|GetSceneCaptureComponent2D) (Variables|/Script/ScoutsOdyssey.PlayerPawn|GetMeshComponent _output_get)))
    (:CastFailed
      (Development|PrintString (Utilities|String|Append (Utilities|GetDisplayName self) " failed to get reference to player pawn!") true true "(R=1.000000,G=0.000000,B=0.000000,A=1.000000)" 1e+01))))

(event EventTick
  (params (DeltaSeconds :type Float%20%28single-precision%29))
  (bind _pawnref (Variables|Default|GetPawnRef))
  (bind _lastenteredsection (Variables|/Script/ScoutsOdyssey.PlayerPawn|GetLastEnteredSection _pawnref))
  ;[1 1 1] Force SceneCaptureComponent to current camera angle transform:
  (Utilities|IsValid _pawnref
    (:Is%20Valid
      (Utilities|IsValid _lastenteredsection
        (:Is%20Valid
          (Transformation|SetWorldTransform (Variables|Default|GetSceneCaptureComponent2D) (Transformation|GetWorldTransform (Variables|/Script/ScoutsOdyssey.StageSectionVolume|GetStageSectionCameraComponent _lastenteredsection)) false false)
          ;[1 1 1] Set SceneCaptureComponent properties to match current camera angle:
          (bind _desiredview (Class|CameraComponent|GetCameraView (Variables|/Script/ScoutsOdyssey.StageSectionVolume|GetStageSectionCameraComponent (Variables|/Script/ScoutsOdyssey.PlayerPawn|GetLastEnteredSection (Variables|Default|GetPawnRef))) 0.0))
          (Variables|/Script/Engine.SceneCaptureComponent2D|SetFOVAngle (Variables|Default|GetSceneCaptureComponent2D) (Utilities|Struct|BreakMinimalViewInfo _desiredview)))))))

(fn ConstructionScript)