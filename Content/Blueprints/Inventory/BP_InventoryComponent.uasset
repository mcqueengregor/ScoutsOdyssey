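; Inventory component that holds a list of item data assets and tracks the current item by index.
; On BeginPlay it fills Items with four hardcoded data assets, including boots, an acorn and a hammer, then binds PrintItem to the OnItemSwitch event.
; PrintItem is debug output that prints a call marker and the display name of the item at CurItemIndex.
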(event Custom|PrintItem
  (Development|PrintString "called!")
  (Development|PrintString (Utilities|GetDisplayName (Utilities|Array|Get(acopy) (Variables|Default|GetItems) (Variables|Default|GetCurItemIndex)))))

(event EventBeginPlay
  (bind _items (Variables|Default|GetItems))
  (Utilities|Array|Add _items "/Game/Blueprints/Inventory/Items/DA_Acorn.DA_Acorn")
  (Utilities|Array|Add _items "/Game/Blueprints/Inventory/Items/DA_DeliciousBoot.DA_DeliciousBoot")
  (Utilities|Array|Add _items "/Game/Blueprints/Inventory/Items/DA_LonelyBoot.DA_LonelyBoot")
  (Utilities|Array|Add _items "/Game/Blueprints/Inventory/Items/DA_PhilbertsHammer.DA_PhilbertsHammer")
  (EventDispatchers|BindEventtoOnItemSwitch (delegate Custom|PrintItem)))