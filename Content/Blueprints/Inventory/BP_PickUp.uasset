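; Pickup actor that the player collects into their inventory component by holding Interact while within its range, then destroys itself.
; Range overlaps toggle input, a gate and an emissive pulse on a dynamic material.
; Holding suspends physics and starts a retriggerable delay that completes the pickup if still held.
; A separate timer, polled by a recursive delayed event, feeds held time to Tick, which shrinks the mesh as progress feedback.
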(event OnComponentBeginOverlap(Pickup_Range)
  (params (OverlappedComponent :type Primitive%20Component%20Object%20Reference) (OtherActor :type Actor%20Object%20Reference) (OtherComp :type Primitive%20Component%20Object%20Reference) (OtherBodyIndex :type Integer) (bFromSweep :type Boolean) (SweepResult :type Hit%20Result%20Structure%20%28by%20ref%29))
  (Utilities|Casting|CastToPlayerPawn OtherActor)
  (Input|EnableInput (Game|GetPlayerController 0))
  ;[1 1 1] Turn glow effect on/off:
  (Rendering|Material|SetScalarParameterValue (Variables|Default|GetDynamicMaterial) "PulseEmissionStrength" 1.0 :!class /Script/Engine.MaterialInstanceDynamic)
  (Utilities|FlowControl|Gate true) ; enters at Open
)

(event OnComponentEndOverlap(Pickup_Range)
  (params (OverlappedComponent :type Primitive%20Component%20Object%20Reference) (OtherActor :type Actor%20Object%20Reference) (OtherComp :type Primitive%20Component%20Object%20Reference) (OtherBodyIndex :type Integer))
  (Utilities|Casting|CastToPlayerPawn OtherActor)
  (Input|DisableInput (Game|GetPlayerController 0))
  ;[1 1 1] Turn glow effect on/off:
  (Rendering|Material|SetScalarParameterValue (Variables|Default|GetDynamicMaterial) "PulseEmissionStrength" 0.0 :!class /Script/Engine.MaterialInstanceDynamic)
  (Utilities|FlowControl|Gate true) ; enters at Close
)

(event Custom|Start%20Timer
  ;[1 1 1] Set Timer for Held time. For Animation. Unrelated to Triggerable Delay => which is used to handle E holding timer
  (bind _returnvalue (Utilities|Time|SetTimerbyEvent (delegate Custom|Start%20Timer) (Variables|Default|GetMaxHeldTime)))
  (Variables|Default|SetTimerHandleRef _returnvalue))

(event Custom|Stop%20Timer
  ;[1 1 1] Set Timer for Held time. For Animation. Unrelated to Triggerable Delay => which is used to handle E holding timer
  (Utilities|Time|PauseTimerbyHandle (Variables|Default|GetTimerHandleRef))
  (Variables|Default|SetTimeHeld 0.0))

(event Custom|Update%20Timer
  ;[1 1 1] Set Timer for Held time. For Animation. Unrelated to Triggerable Delay => which is used to handle E holding timer
  ;;[1 1 1] Looping function on its own. Recursive with time wait.
  (if (Variables|Default|GetIsHeld)
    (Variables|Default|SetTimeHeld (Class|KismetSystemLibrary|GetTimerElapsedTimeHandle (Variables|Default|GetTimerHandleRef)))
    (Utilities|FlowControl|Delay 0.1)
    (CallFunction|UpdateTimer)
    (else
      (CallFunction|StopTimer))))

(event Custom|PickupEffect
  (bind _percentage (CallFunction|GetHeldPercentage))
  (Transformation|SetRelativeScale3D (Variables|Default|GetPlane) (* (Math|Conversions|ToVector(Float) (- 1.0 _percentage)) 0.2)))

(event EventBeginPlay
  (Input|EnableInput (Game|GetPlayerController 0))
  ;[1 1 1] Create dynamic material instance on game startup, store reference to it so that parameters can be adjusted during gameplay:
  (bind _returnvalue (Rendering|Material|CreateDynamicMaterialInstance (Rendering|Material|GetMaterial (Variables|Default|GetPlane) 0) "None" "None" :!class /Script/Engine.KismetMaterialLibrary))
  (bind _output_get (Variables|Default|SetDynamicMaterial _returnvalue))
  (Rendering|Material|SetMaterial (Variables|Default|GetPlane) 0 _output_get))

(event EventTick
  (params (DeltaSeconds :type Float%20%28single-precision%29))
  (CallFunction|PickupEffect))

(event EventPickup
  (params (Inventory :type Inventory%20Component%20Object%20Reference))
  (Class|InventoryComponent|AddItem Inventory (Variables|Default|GetItemToPickup)))

(event Input|ActionEvents|InputActionInteract
  (params (Key :type Key%20Structure :default "None"))
  (bind _plane (Variables|Default|GetPlane))
  (:Pressed
    (Physics|SetSimulatePhysics _plane false)
    (Variables|Default|SetIsHeld true)
    (Utilities|FlowControl|Gate true
      (:Exit
        (Utilities|FlowControl|Sequence
          (:then_0
            (Utilities|FlowControl|RetriggerableDelay (Variables|Default|GetMaxHeldTime))
            (if (Variables|Default|GetIsHeld)
              (bind _asbp_player_pawn (Utilities|Casting|CastToBP_PlayerPawn (Game|Player|GetPlayerPawn 0)))
              (CallFunction|Pickup (Variables|/Game/Blueprints/DefaultActors/BP_PlayerPawn.BP_PlayerPawn_C|GetBP_InventoryComponent _asbp_player_pawn))
              (Actor|DestroyActor)))
          (:then_1
            (CallFunction|StartTimer)
            (CallFunction|UpdateTimer))))))
  (:Released
    (Physics|SetSimulatePhysics _plane true)
    (Variables|Default|SetIsHeld false)))

(fn ConstructionScript)

(fn GetHeldPercentage
  (return (/ (Variables|Default|GetTimeHeld) (Variables|Default|GetMaxHeldTime))))