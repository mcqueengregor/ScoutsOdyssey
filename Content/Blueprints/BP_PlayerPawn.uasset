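; BP_PlayerPawn is a player pawn that lets the player cycle through inventory items with the mouse scroll wheel.
; The MouseScroll axis value is truncated, added to the inventory component's CurItemIndex and clamped to the Items array bounds.
; The component's OnItemSwitch is then called behind an always-true branch, so it fires on every axis update, even when the index is unchanged.
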(event Input|AxisEvents|InputAxisMouseScroll
  (params (AxisValue :type Float%20%28single-precision%29))
  (bind _bp_inventorycomponent (Variables|Default|GetBP_InventoryComponent))
  (Variables|/Game/Blueprints/Inventory/BP_InventoryComponent.BP_InventoryComponent_C|SetCurItemIndex _bp_inventorycomponent (Math|Integer|Clamp(Integer) (+ (Math|Float|Truncate AxisValue) (Variables|/Game/Blueprints/Inventory/BP_InventoryComponent.BP_InventoryComponent_C|GetCurItemIndex _bp_inventorycomponent)) 0 (- (Utilities|Array|Length (Variables|/Game/Blueprints/Inventory/BP_InventoryComponent.BP_InventoryComponent_C|GetItems _bp_inventorycomponent)) 1)))
  (if true
    (Default|CallOnItemSwitch (Variables|Default|GetBP_InventoryComponent))))

(fn ConstructionScript)