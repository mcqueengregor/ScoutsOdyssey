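; BP_HoneyTreeInteract is an interactable honey tree that plays dialogue in response to beehive interaction results.
; On BeginPlay it binds to the BeehiveInteract component's fail-to-interact and honey boot collected events.
; A failed interaction starts the current dialogue through BPDialogueComponent.
; Collecting the honey boot switches DialogueTree to BT_GotHoney, resets HasTriggered and restarts dialogue so the new conversation plays.
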(event Custom|OnFailToInteract_Event_0
  (Class|DialogueComponent|StartDialogue (Variables|Default|GetBP_DialogueComponent)))

(event Custom|OnHoneyBootCollected
  (bind _bp_dialoguecomponent (Variables|Default|GetBP_DialogueComponent))
  (Variables|Default|SetDialogueTree "/Game/Blueprints/Dialogue/DialogueTrees/BT_GreenHouseArea/BT_GotHoney.BT_GotHoney")
  (Variables|/Script/ScoutsOdyssey.DialogueComponent|SetHasTriggered _bp_dialoguecomponent false)
  (Class|DialogueComponent|StartDialogue _bp_dialoguecomponent))

(event EventBeginPlay
  (EventDispatchers|AssignOnFailtoInteract (Variables|Default|GetBeehiveInteract) (delegate Custom|OnFailToInteract_Event_0))
  (EventDispatchers|BindEventtoOnHoneyBootCollected (Variables|Default|GetBeehiveInteract) (delegate Custom|OnHoneyBootCollected)))

(fn ConstructionScript)