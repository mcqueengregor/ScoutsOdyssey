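; Big tree actor that reveals a linked small tree and its acorn pickup once the tree disappears.
; On BeginPlay it binds to TreeInteract's OnTreeDisappear and makes the small tree's child-actor acorn static, without physics or pickup collision.
; The disappear event shows the small tree mesh and acorn plane and restores the pickup's overlap collision.
; The node hiding the small tree mesh is disconnected, so initial visibility is not set here.
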(event Custom|OnTreeDisappear
  (bind _smalltreeactor (Variables|Default|GetSmallTreeActor))
  (Rendering|SetVisibility (Variables|/Game/Blueprints/DefaultActors/BP_SmallTree.BP_SmallTree_C|GetStaticMesh _smalltreeactor) true false)
  (bind _asbp_acorn_pickup (Utilities|Casting|CastToBP_AcornPickup (Variables|/Script/Engine.ChildActorComponent|GetChildActor (Variables|/Game/Blueprints/DefaultActors/BP_SmallTree.BP_SmallTree_C|GetAcornPickup _smalltreeactor))))
  (Rendering|SetVisibility (Variables|/Game/Blueprints/Inventory/BP_PickUp.BP_Pickup_C|GetPlane _asbp_acorn_pickup) true false)
  (Collision|SetCollisionProfileName (Variables|/Game/Blueprints/Inventory/BP_PickUp.BP_Pickup_C|GetPickup_Range _asbp_acorn_pickup) "OverlapAllDynamic" true :!class /Script/Engine.PrimitiveComponent))

(event EventBeginPlay
  ;[1 1 1] Force physics off on small tree's acorn pickup, hide plane meshes:
  (EventDispatchers|BindEventtoOnTreeDisappear (Variables|Default|GetTreeInteract) (delegate Custom|OnTreeDisappear))
  (bind _asbp_acorn_pickup (Utilities|Casting|CastToBP_AcornPickup (Variables|/Script/Engine.ChildActorComponent|GetChildActor (Variables|/Game/Blueprints/DefaultActors/BP_SmallTree.BP_SmallTree_C|GetAcornPickup (Variables|Default|GetSmallTreeActor)))))
  (Variables|/Game/Blueprints/Inventory/BP_PickUp.BP_Pickup_C|SetIsStatic _asbp_acorn_pickup true)
  (Physics|SetSimulatePhysics (Variables|/Game/Blueprints/Inventory/BP_PickUp.BP_Pickup_C|GetPlane _asbp_acorn_pickup) false)
  (Collision|SetCollisionProfileName (Variables|/Game/Blueprints/Inventory/BP_PickUp.BP_Pickup_C|GetPickup_Range _asbp_acorn_pickup) "NoCollision" true :!class /Script/Engine.PrimitiveComponent))

(fn ConstructionScript)