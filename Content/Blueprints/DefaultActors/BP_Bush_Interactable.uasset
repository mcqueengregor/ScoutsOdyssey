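; Interactable bush actor that hands dialogue character status over to Philbert when it disappears.
; On BeginPlay it caches the DialogueComponent from its Philbert reference and flags its own dialogue component as a character.
; Tick polls BushInteract's IsDisappearing state, then sets IsCharacter on Philbert's component and clears it on the bush.
; The check on Philbert's flag skips the swap while he is already marked.
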(event EventBeginPlay
  (Variables|Default|SetPhilbertDialogueComponentRef (Actor|GetComponentbyClass (Variables|Default|GetPhilbertRef) "/Script/ScoutsOdyssey.DialogueComponent"))
  (Variables|/Script/ScoutsOdyssey.DialogueComponent|SetbIsCharacter (Variables|Default|GetBP_DialogueComponent) true))

(event EventTick
  (params (DeltaSeconds :type Float%20%28single-precision%29))
  (bind _philbertdialoguecomponentref (Variables|Default|GetPhilbertDialogueComponentRef))
  (if (Math|Boolean|ANDBoolean (Utilities|IsValid _philbertdialoguecomponentref) (not (Variables|/Script/ScoutsOdyssey.DialogueComponent|GetbIsCharacter _philbertdialoguecomponentref)) (Variables|/Script/ScoutsOdyssey.BushInteractComponent|GetbIsDisappearing (Variables|Default|GetBushInteract)))
    (Variables|/Script/ScoutsOdyssey.DialogueComponent|SetbIsCharacter (Variables|Default|GetPhilbertDialogueComponentRef) true)
    (Variables|/Script/ScoutsOdyssey.DialogueComponent|SetbIsCharacter (Variables|Default|GetBP_DialogueComponent) false)))

(fn ConstructionScript)