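; Stage teleport trigger volume that, as written, only prepares a fade-to-black post process material; it contains no teleport or fade logic.
; On BeginPlay it finds a PostProcessVolume and assumes its last blendable is the fade Material.
; It swaps that entry for a stored dynamic instance, rebuilding the volume's settings from the materials array alone.
; A failed Material cast prints an error, and parent BeginPlay is never called.
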(event EventBeginPlay
  ;[1 1 1] Get settings from global post process volume, find "fade to black" post process material and append dynamic version to post process volume rendering features list:
  (bind _returnvalue (Actor|GetActorOfClass "/Script/Engine.PostProcessVolume"))
  (CallFunction|AppendDynamicFadetoBlack _returnvalue))

(event EventSetupDynamicFadetoBlackMat)

(fn ConstructionScript)

(fn GetFadetoBlackMatRef
  (return))

(fn AppendDynamicFadetoBlack
  (params (PostProcessVolumeRef :type Post%20Process%20Volume%20Object%20Reference))
  (bind _output_get (LocalVariables|SetWeightedBlendablesArrayRef (Utilities|Struct|BreakWeightedBlendables (Utilities|Struct|BreakPostProcessSettings (Variables|/Script/Engine.PostProcessVolume|GetSettings PostProcessVolumeRef)))))
  (bind _asmaterial (Utilities|Casting|CastToMaterial (.Object (Utilities|Struct|BreakWeightedBlendable (Utilities|Array|Get(acopy) _output_get (Utilities|Array|LastIndex (Utilities|Struct|BreakWeightedBlendables (Utilities|Struct|BreakPostProcessSettings (Variables|/Script/Engine.PostProcessVolume|GetSettings PostProcessVolumeRef))))))))
    (:then
      (bind _output_get_2 (LocalVariables|SetFadeToBlackMaterialRef _asmaterial))
      (bind _returnvalue (Rendering|Material|CreateDynamicMaterialInstance _output_get_2 "None" "None" :!class /Script/Engine.KismetMaterialLibrary))
      (Utilities|Array|RemoveIndex (LocalVariables|GetWeightedBlendablesArrayRef) (Utilities|Array|LastIndex (LocalVariables|GetWeightedBlendablesArrayRef)))
      (Utilities|Array|AppendArray (LocalVariables|GetWeightedBlendablesArrayRef) (Utilities|Array|MakeArray (Utilities|Struct|MakeWeightedBlendable 1.0 _returnvalue)))
      (Variables|/Script/Engine.PostProcessVolume|SetSettings PostProcessVolumeRef (Utilities|Struct|MakePostProcessSettings (Utilities|Struct|MakeWeightedBlendables (LocalVariables|GetWeightedBlendablesArrayRef))))
      (Variables|Default|SetFadeToBlackMaterialDynamic _returnvalue)
      (return))
    (:CastFailed
      (Development|PrintString "Failed to retrieve reference to fade to black material!" true true "(R=1.000000,G=0.000000,B=0.000000,A=1.000000)" 1e+01))))