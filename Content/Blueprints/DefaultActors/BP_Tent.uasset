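; BP_Tent is a tent actor that triggers dialogue in response to player-facing events.
; It binds to TentInteract's all-built and failed-interaction events, swapping in the matching dialogue tree for BPDialogueComponent.
; PropCollider overlap starts the current dialogue, then switches the tree to the fail-to-interact one.
; Boolean flags make overlap and failure dialogues one-shot, each also playing a level sequence named for disabling it.
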(event OnComponentBeginOverlap(PropCollider)
  (params (OverlappedComponent :type Primitive%20Component%20Object%20Reference) (OtherActor :type Actor%20Object%20Reference) (OtherComp :type Primitive%20Component%20Object%20Reference) (OtherBodyIndex :type Integer) (bFromSweep :type Boolean) (SweepResult :type Hit%20Result%20Structure%20%28by%20ref%29))
  ;[1 1 1] On Collision Enter
  (if (Variables|Default|GetCollisionCanTriggerConversation)
    (Class|DialogueComponent|StartDialogue (Variables|Default|GetBP_DialogueComponent))
    (Variables|Default|SetCollisionCanTriggerConversation false)
    (bind _returnvalue (Sequencer|Player|CreateLevelSequencePlayer "/Game/LevelSequences/TutorialStart/DisableTentConversation/LS_DisableTentCollisionDialogue.LS_DisableTentCollisionDialogue"))
    (Sequencer|Player|Play _returnvalue :!class /Script/MovieScene.MovieSceneSequencePlayer)
    (Variables|/Script/ScoutsOdyssey.DialogueComponent|SetHasTriggered (Variables|Default|GetBP_DialogueComponent) false)
    (Variables|Default|SetDialogueTree (Variables|Default|GetFailToInteractDialogue))))

(event Custom|OnAllTentBuilt_Event_0
  ;[1 1 1] On All Tent Built Binding
  (Variables|Default|SetDialogueTree (Variables|Default|GetAllTentBuildDialogue))
  (Class|DialogueComponent|StartDialogue (Variables|Default|GetBP_DialogueComponent)))

(event Custom|OnFailToInteract_0
  ;[1 1 1] On Fail To Interact Binding
  (if (Variables|Default|GetFailInteractCanTriggerConversation)
    (Variables|Default|SetDialogueTree (Variables|Default|GetFailToInteractDialogue))
    (Class|DialogueComponent|StartDialogue (Variables|Default|GetBP_DialogueComponent))
    (Variables|Default|SetFailInteractCanTriggerConversation false)
    (bind _returnvalue (Sequencer|Player|CreateLevelSequencePlayer "/Game/LevelSequences/TutorialStart/DisableTentConversation/LS_DisableFailInteractDialogue.LS_DisableFailInteractDialogue"))
    (Sequencer|Player|Play _returnvalue :!class /Script/MovieScene.MovieSceneSequencePlayer)))

(event Custom|DisableCollisionEnterDialogue
  ;[1 1 1] On Collision Enter
  (Variables|Default|SetCollisionCanTriggerConversation false))

(event Custom|DisableFailToInteractDialogue
  ;[1 1 1] On Fail To Interact Binding
  (Variables|Default|SetFailInteractCanTriggerConversation false))

(event EventBeginPlay
  (Variables|/Script/ScoutsOdyssey.DialogueComponent|SetHasTriggered (Variables|Default|GetBP_DialogueComponent) false)
  (Variables|Default|SetCollisionCanTriggerConversation true)
  (Variables|Default|SetFailInteractCanTriggerConversation true)
  ;[1 1 1] On All Tent Built Binding
  (EventDispatchers|AssignOnAllTentBuilt (Variables|Default|GetTentInteract) (delegate Custom|OnAllTentBuilt_Event_0))
  ;[1 1 1] On Fail To Interact Binding
  (EventDispatchers|BindEventtoOnFailtoInteract (Variables|Default|GetTentInteract) (delegate Custom|OnFailToInteract_0)))

(fn ConstructionScript)